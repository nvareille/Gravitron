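; Monster actor that moves along a path and bumps the player away on contact.
; A timeline started on BeginPlay lerps its location from StartPosition, captured in the construction script, to EndPosition.
; When the player character overlaps the BumpCollider sphere, sized by ColliderRadius, it stops their movement, launches them along EjectDirection and plays a bump sound.
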(event `self.ReceiveBeginPlay`
  (bind (_direction _movement) (`Timeline|Timeline_0` :!via `PlayFromStart`)
    (:`Update`
      (`self.K2_SetActorLocation` (`KismetMathLibrary.VLerp` (`self.StartPosition`) (`self.EndPosition`) _movement)))))

(event `self.BumpCollider.OnComponentBeginOverlap`
  (params (OtherActor :type "Actor Object Reference") (OtherComp :type "PrimitiveComponent Object Reference") (OtherBodyIndex :type Integer) (bFromSweep :type Boolean) (SweepResult :type "HitResult Structure (by ref)"))
  (bind _returnvalue (`GameplayStatics.GetPlayerCharacter` 0))
  (if (== OtherActor _returnvalue)
    (`MovementComponent.StopMovementImmediately` (`Character.CharacterMovement` _returnvalue))
    (`Character.LaunchCharacter` _returnvalue (`self.EjectDirection`) false false)
    (`GameplayStatics.PlaySound2D` (`self.BumpSound`))))

(fn `UserConstructionScript`
  (`SphereComponent.SetSphereRadius` (`self.BumpCollider`) (`self.ColliderRadius`) true)
  (set `self.StartPosition` (`self.K2_GetActorLocation`)))