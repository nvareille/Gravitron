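; Parent pickup Blueprint for collectibles that spin in place and are collected when the player touches them.
; The construction script applies a configurable static mesh, position offset and uniform scale to the pickup mesh.
; Tick applies a framerate-independent yaw rotation scaled by a speed multiplier.
; On overlap with the player character, it destroys itself, plays a 2D sound and reports its Type to the ScoreManager.
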(event `self.ReceiveTick`
  (params (DeltaSeconds :type "Float (single-precision)"))
  ;[1 1 1] Rotation
  (`self.K2_AddActorLocalRotation` (`KismetMathLibrary.MakeRotator` 0.0 0.0 (* DeltaSeconds (`self.RotationSpeedMultiplier`)))))

(event `self.Pickup_Collider.OnComponentBeginOverlap`
  (params (OtherActor :type "Actor Object Reference") (OtherComp :type "PrimitiveComponent Object Reference") (OtherBodyIndex :type Integer) (bFromSweep :type Boolean) (SweepResult :type "HitResult Structure (by ref)"))
  ;[1 1 1] Collision Condition
  (if (== OtherActor (`GameplayStatics.GetPlayerCharacter` 0))
    ;[1 1 1] Collision Effects
    (`self.K2_DestroyActor`)
    (`GameplayStatics.PlaySound2D` (`self.PickupSound`))
    ;[1 1 1] Set score
    (`/Game/Blueprints/ScoreManager.SetNewPickup` (`self.ScoreManager`) (`self.Type`))))

(fn `UserConstructionScript`
  (bind _scalemultiplier (`self.ScaleMultiplier`))
  (bind _pickup_mesh (`self.Pickup_Mesh`))
  (`StaticMeshComponent.SetStaticMesh` _pickup_mesh (`self.StaticMesh`))
  (`SceneComponent.K2_AddLocalOffset` _pickup_mesh (`self.PositionOffset`) false false)
  (`SceneComponent.SetWorldScale3D` _pickup_mesh (`KismetMathLibrary.MakeVector` _scalemultiplier _scalemultiplier _scalemultiplier)))