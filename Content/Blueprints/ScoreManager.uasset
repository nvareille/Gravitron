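; ScoreManager tracks collected pickups and shows them on the HUD.
; On BeginPlay it creates the HUD widget, hands it a reference to itself and adds it to the viewport.
; SetNewPickup matches a type string against a fixed set of pickup names, then increments the pickup count and tells the HUD to switch on the matching element.
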(event `self.ReceiveBeginPlay`
  ;[1 1 1] Set HUD
  (bind _returnvalue (`|CreateWidget` "/Game/Blueprints/HUD.HUD_C"))
  (bind _output_get (set `self.HUD` _returnvalue))
  (set `/Game/Blueprints/HUD.ScoreManager` self _output_get)
  (`UserWidget.AddToViewport` _output_get 0))

(fn `SetNewPickup`
  (params (type :type String))
  ;[1 1 1] Find Pickup Type
  (if (== type "vial")
    ;[1 1 1] Add Pickup Nb
    (`/Engine/EditorBlueprintResources/StandardMacros.IncrementInt` (`self.PickupNb`) :!label _label
      (:`  `
        (`/Game/Blueprints/HUD.SetElementOn` (`self.HUD`) type)))
    (elif (== type "bridge")
      (goto _label)
      (elif (== type "monster")
        (goto _label)
        (elif (== type "snack")
          (goto _label)
          (elif (== type "picture")
            (goto _label)
            (elif (== type "exam")
              (goto _label)
              (elif (== type "friend")
                (goto _label)))))))))

(fn `UserConstructionScript`)