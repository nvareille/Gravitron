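; End is a trigger volume actor that starts an ending cinematic when the player walks into it.
; On actor overlap with player character 0, it plays EndCinematic and stops the audio component of the referenced Music actor.
; The construction script sizes the Collider box from the ColliderSize variable.
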(event `self.ReceiveActorBeginOverlap`
  (params (OtherActor :type "Actor Object Reference"))
  ;[1 1 1] Collider Check
  (if (== OtherActor (`GameplayStatics.GetPlayerCharacter` 0))
    (`MatineeActor.Play` (`self.EndCinematic`))
    (`AudioComponent.Stop` (`AmbientSound.AudioComponent` (`self.Music`)))))

(fn `UserConstructionScript`
  (`BoxComponent.SetBoxExtent` (`self.Collider`) (`self.ColliderSize`) true))